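; BP_Tower is an enemy tower whose destruction counts toward opening a boss door.
; On BeginPlay it caches its WBP_UITower widget, ignores pushes and resets its inherited enemy stats.
; The damage hook updates the widget's life bar from the Life to MaxLife ratio.
; The death hook passes DammageToSystem to the controller's UI system and asks CurrentBossDoor to check whether to open.
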(event `self.ReceiveBeginPlay`
  (`parent.ReceiveBeginPlay`)
  (bind _aswbp_uitower (cast `/Game/Blueprint/Enemy_Tower/Tower/WBP_UITower` (`WidgetComponent.GetWidget` (`self.Widget`))))
  (set `self.uiTower` _aswbp_uitower)
  (set `self.ignorePush` true)
  (`self.ResetStatsEnemy`))

(fn `AddEffectDammage`
  (`/Game/Blueprint/Enemy_Tower/Tower/WBP_UITower.setTowerUILife` (`self.uiTower`) (/ (`KismetMathLibrary.Conv_IntToDouble` (`self.life`)) (`KismetMathLibrary.Conv_IntToDouble` (`self.maxLife`)))))

(fn `AddEffectDead`
  (`/Game/Blueprint/WBP_UISystem.setUISystem` (`/Game/Blueprint/BP_PlayerController.uiSystem` (`/Game/Blueprint/FunctionLibrary/FCL_GetController.GetControllerAs`)) (`self.dammageToSystem`))
  (`/Game/Blueprint/Enemy_Tower/Tower/BP_BossDoor.CheckOpenDoor` (`self.currentBossDoor`)))

(fn `UserConstructionScript`
  (`parent.UserConstructionScript`))