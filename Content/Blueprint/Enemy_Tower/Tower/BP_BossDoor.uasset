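; BP_BossDoor is a boss door actor that counts down the towers left to destroy.
; When CheckOpenDoor brings the count to zero, it blends the player's camera to itself, disables input and destroys every BP_Enemy.
; The delayed camera return and input re-enable sit inside the enemy loop, so they run only if an enemy exists.
; The graph contains no door-opening movement.
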(event `CheckOpenDoor`
  (bind _numbertowertodestroy (`self.numberTowerToDestroy`))
  (`/Engine/EditorBlueprintResources/StandardMacros.DecrementInt` _numbertowertodestroy
    (:`  `
      (if (<= _numbertowertodestroy 0)
        (`PlayerController.SetViewTargetWithBlend` (`/Game/Blueprint/FunctionLibrary/FCL_GetController.GetControllerAs`) self 1.0 "VTBlend_Linear" 0.0 false)
        (`self.DisableInput` (`/Game/Blueprint/FunctionLibrary/FCL_GetCharacter.GetCharacterAs`) null)
        (bind _outactors (`GameplayStatics.GetAllActorsOfClass` "/Game/Blueprint/Enemy_Tower/BP_Enemy.BP_Enemy_C"))
        (for _array_element _outactors
          (`self.K2_DestroyActor` _array_element)
          (`KismetSystemLibrary.Delay` 2.0)
          (`PlayerController.SetViewTargetWithBlend` (`/Game/Blueprint/FunctionLibrary/FCL_GetController.GetControllerAs`) (`/Game/Blueprint/FunctionLibrary/FCL_GetCharacter.GetCharacterAs`) 1.0 "VTBlend_Linear" 0.0 false)
          (`self.EnableInput` (`/Game/Blueprint/FunctionLibrary/FCL_GetCharacter.GetCharacterAs`) null))))))

(fn `UserConstructionScript`)