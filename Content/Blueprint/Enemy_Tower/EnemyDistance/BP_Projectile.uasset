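; Projectile for the ranged tower enemy that flies at the player and damages them on contact.
; On spawn it rotates to face away from the character and moves backward along its forward vector each tick, without homing, sweep or delta-time scaling.
; Cube overlap with the ThirdPersonCharacter reduces life through the controller if damage is allowed, then destroys the projectile, which otherwise expires after a short lifespan.
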(event `self.ReceiveBeginPlay`
  (`self.K2_SetActorRotation` (`KismetMathLibrary.FindLookAtRotation` (`self.K2_GetActorLocation` (`/Game/Blueprint/FunctionLibrary/FCL_GetCharacter.GetCharacterAs`)) (`self.K2_GetActorLocation`)))
  (`self.SetLifeSpan` 1.0))

(event `self.ReceiveTick`
  (params (DeltaSeconds :type "Float (single-precision)"))
  (`self.K2_SetActorLocation` (+ (`self.K2_GetActorLocation`) (* (`self.GetActorForwardVector`) -12.5))))

(event `self.Cube.OnComponentBeginOverlap`
  (params (OverlappedComponent :type "PrimitiveComponent Object Reference") (OtherActor :type "Actor Object Reference") (OtherComp :type "PrimitiveComponent Object Reference") (OtherBodyIndex :type Integer) (bFromSweep :type Boolean) (SweepResult :type "HitResult Structure (by ref)"))
  (bind _asbp_player_controller (`/Game/Blueprint/FunctionLibrary/FCL_GetController.GetControllerAs`))
  (cast `/Game/Blueprint/ThirdPersonCharacter` OtherActor)
  (if (`/Game/Blueprint/BP_PlayerController.canTakeDammage` _asbp_player_controller)
    (`/Game/Blueprint/BP_PlayerController.ChangeLife` _asbp_player_controller -4)
    (`self.K2_DestroyActor`)))

(fn `UserConstructionScript`)