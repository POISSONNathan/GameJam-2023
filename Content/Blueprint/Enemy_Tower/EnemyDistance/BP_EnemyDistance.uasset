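; BP_EnemyDistance is a ranged enemy that chases the player character and fires projectiles once within 700 units.
; While CanMove is set, Tick faces the target, then either follows with SimpleMoveToActor or stops and attacks, toggling IsAttack on ABP_Distance to match.
; A Delay inside Tick paces BP_Projectile spawns, with the Shot flag cancelling a pending shot if the target moves out of range.
; BeginPlay sets MaxLife and resets enemy stats.
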(event `self.ReceiveBeginPlay`
  (set `self.maxLife` 4)
  (`self.ResetStatsEnemy`))

(event `self.ReceiveTick`
  (params (DeltaSeconds :type "Float (single-precision)"))
  (if (`self.canMove`)
    (`self.K2_SetActorRotation` (`KismetMathLibrary.FindLookAtRotation` (`self.K2_GetActorLocation`) (`self.K2_GetActorLocation` (`/Game/Blueprint/FunctionLibrary/FCL_GetCharacter.GetCharacterAs`))))
    (if (>= (`KismetMathLibrary.Vector_Distance` (`self.K2_GetActorLocation` (`/Game/Blueprint/FunctionLibrary/FCL_GetCharacter.GetCharacterAs`)) (`self.K2_GetActorLocation`)) 700.0)
      (`AIBlueprintHelperLibrary.SimpleMoveToActor` (`self.GetController`) (`/Game/Blueprint/FunctionLibrary/FCL_GetCharacter.GetCharacterAs`))
      (set `self.currentPos` (`self.K2_GetActorLocation`))
      (set `self.shot` false)
      (bind _asabp_distance (cast `/Game/Blueprint/Mesh/DistanceMESH/ABP_Distance` (`SkeletalMeshComponent.GetAnimInstance` (`self.Mesh`))))
      (set `/Game/Blueprint/Mesh/DistanceMESH/ABP_Distance.isAttack` false _asabp_distance)
      (else
        (`Controller.StopMovement` (`self.GetController`))
        (set `self.shot` true)
        (bind _asabp_distance_2 (cast `/Game/Blueprint/Mesh/DistanceMESH/ABP_Distance` (`SkeletalMeshComponent.GetAnimInstance` (`self.Mesh`))))
        (set `/Game/Blueprint/Mesh/DistanceMESH/ABP_Distance.isAttack` true _asabp_distance_2)
        (`KismetSystemLibrary.Delay` 0.9)
        (if (`self.shot`)
          (`|SpawnActorFromClass` "/Game/Blueprint/Enemy_Tower/EnemyDistance/BP_Projectile.BP_Projectile_C" (`self.GetTransform`) "Undefined" "OverrideRootScale" null null))))))

(fn `UserConstructionScript`
  (`parent.UserConstructionScript`))