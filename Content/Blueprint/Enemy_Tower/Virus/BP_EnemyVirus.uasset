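; BP_EnemyVirus is a virus enemy that chases the player and bursts when the player gets close.
; Tick drives movement toward the player character until a TriggerZone overlap sets Explode.
; It then flags the attack animation and, after a short Delay, spawns a BP_EnemyVirusZone with an explosion effect before resuming the chase.
; Its AddEffectDead function spawns a BP_EnemyVirusMini1 above its position.
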(event `self.ReceiveBeginPlay`
  (`SceneComponent.SetVisibility` (`self.Sphere`) false false)
  (set `self.maxLife` 3)
  (`self.ResetStatsEnemy`)
  (set `self.ignorePush` true))

(event `self.ReceiveTick`
  (params (DeltaSeconds :type "Float (single-precision)"))
  (if (`self.canMove`)
    (if (`self.explode`)
      (bind _asabp_virus (cast `/Game/Blueprint/Mesh/VirusMESH/ABP_Virus` (`SkeletalMeshComponent.GetAnimInstance` (`self.Mesh`))))
      (set `/Game/Blueprint/Mesh/VirusMESH/ABP_Virus.isAttack` true _asabp_virus)
      (`KismetSystemLibrary.Delay` 1.0)
      (`|SpawnActorFromClass` "/Game/Blueprint/Enemy_Tower/Virus/BP_EnemyVirusZone.BP_EnemyVirusZone_C" (`SceneComponent.K2_GetComponentToWorld` (`self.Sphere`)) "Undefined" "OverrideRootScale" null null)
      (`GameplayStatics.SpawnEmitterAtLocation` "/Game/StarterContent/Particles/P_Explosion.P_Explosion" (`self.K2_GetActorLocation`) (struct) (5.0 5.0 1.0))
      (set `self.explode` false)
      (else
        (`AIBlueprintHelperLibrary.SimpleMoveToActor` (`self.GetController`) (`/Game/Blueprint/FunctionLibrary/FCL_GetCharacter.GetCharacterAs`))
        (bind _asabp_virus_2 (cast `/Game/Blueprint/Mesh/VirusMESH/ABP_Virus` (`SkeletalMeshComponent.GetAnimInstance` (`self.Mesh`))))
        (set `/Game/Blueprint/Mesh/VirusMESH/ABP_Virus.isAttack` false _asabp_virus_2)))))

(event `self.TriggerZone.OnComponentBeginOverlap`
  (params (OverlappedComponent :type "PrimitiveComponent Object Reference") (OtherActor :type "Actor Object Reference") (OtherComp :type "PrimitiveComponent Object Reference") (OtherBodyIndex :type Integer) (bFromSweep :type Boolean) (SweepResult :type "HitResult Structure (by ref)"))
  (cast `/Game/Blueprint/ThirdPersonCharacter` OtherActor)
  (set `self.explode` true))

(fn `AddEffectDead`
  (`AIBlueprintHelperLibrary.SpawnAIFromClass` "/Game/Blueprint/Enemy_Tower/Virus/BP_EnemyVirusMini1.BP_EnemyVirusMini1_C" null (+ (`self.K2_GetActorLocation`) (0.0 0.0 100.0)) (struct) false null))

(fn `UserConstructionScript`
  (`parent.UserConstructionScript`))