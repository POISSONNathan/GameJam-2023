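; Mini virus enemy that chases the character and releases a virus zone with an explosion effect when the player gets close.
; On BeginPlay it hides its sphere, sets a low max life, resets inherited enemy stats and ignores pushes.
; While movable, Tick drives simple move-to-actor until a trigger overlap sets Explode, then spawns both after a short delay and clears the flag.
; The death-effect function is empty.
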(event `self.ReceiveBeginPlay`
  (`SceneComponent.SetVisibility` (`self.Sphere`) false false)
  (set `self.maxLife` 3)
  (`self.ResetStatsEnemy`)
  (set `self.ignorePush` true))

(event `self.ReceiveTick`
  (params (DeltaSeconds :type "Float (single-precision)"))
  (if (`self.canMove`)
    (if (`self.explode`)
      (`KismetSystemLibrary.Delay` 1.5)
      (`|SpawnActorFromClass` "/Game/Blueprint/Enemy_Tower/Virus/BP_EnemyVirusZone.BP_EnemyVirusZone_C" (`SceneComponent.K2_GetComponentToWorld` (`self.Sphere`)) "Undefined" "OverrideRootScale" null null)
      (`GameplayStatics.SpawnEmitterAtLocation` "/Game/StarterContent/Particles/P_Explosion.P_Explosion" (`self.K2_GetActorLocation`) (struct) (5.0 5.0 1.0))
      (set `self.explode` false)
      (else
        (`AIBlueprintHelperLibrary.SimpleMoveToActor` (`self.GetController`) (`/Game/Blueprint/FunctionLibrary/FCL_GetCharacter.GetCharacterAs`))))))

(event `self.TriggerZone.OnComponentBeginOverlap`
  (params (OverlappedComponent :type "PrimitiveComponent Object Reference") (OtherActor :type "Actor Object Reference") (OtherComp :type "PrimitiveComponent Object Reference") (OtherBodyIndex :type Integer) (bFromSweep :type Boolean) (SweepResult :type "HitResult Structure (by ref)"))
  (cast `/Game/Blueprint/ThirdPersonCharacter` OtherActor)
  (set `self.explode` true))

(fn `AddEffectDead`)

(fn `UserConstructionScript`
  (`parent.UserConstructionScript`))