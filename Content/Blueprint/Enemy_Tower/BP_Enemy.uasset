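; Base enemy Character that handles health, damage, death and knockback.
; Taking damage lowers Life and calls a hit-effect hook; at zero it calls a death-effect hook, decrements the controller's enemy count and destroys itself, with both hooks left empty here.
; Unless IgnorePush is set, a push stops AI movement, launches it away from another character with unnormalized, distance-scaled velocity, and briefly clears CanMove.
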(event `ResetStatsEnemy`
  (set `self.life` (`self.maxLife`)))

(event `TakeDammage`
  (params (AmmountOfDammage :type Integer))
  (bind _output_get (set `self.life` (- (`self.life`) AmmountOfDammage)))
  (`self.AddEffectDammage`)
  (if (<= _output_get 0)
    (`self.AddEffectDead`)
    (`/Engine/EditorBlueprintResources/StandardMacros.DecrementInt` (`/Game/Blueprint/BP_PlayerController.numberEnemyOnMap` (`/Game/Blueprint/FunctionLibrary/FCL_GetController.GetControllerAs`))
      (:`  `
        (`self.K2_DestroyActor`)))))

(event `GetPushed`
  (if (not (`self.ignorePush`))
    (set `self.canMove` false)
    (`Controller.StopMovement` (`self.GetController`))
    (`self.LaunchCharacter` (* (- (`self.K2_GetActorLocation` (`/Game/Blueprint/FunctionLibrary/FCL_GetCharacter.GetCharacterAs`)) (`self.K2_GetActorLocation`)) -100.0))
    (`KismetSystemLibrary.Delay` 0.2)
    (set `self.canMove` true)))

(fn `AddEffectDammage`)

(fn `AddEffectDead`)

(fn `UserConstructionScript`)