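; BP_EnemyTurn is an enemy that chases the player character and affects its life on contact.
; On begin play it sets its max life and resets its enemy stats.
; Each tick it uses simple AI move-to toward the character while CanMove is set, and stops movement otherwise.
; A sphere overlap with the third-person character passes the Dammage value to the controller's ChangeLife.
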(event `self.ReceiveBeginPlay`
  (set `self.maxLife` 2)
  (`self.ResetStatsEnemy`))

(event `self.ReceiveTick`
  (params (DeltaSeconds :type "Float (single-precision)"))
  (if (`self.canMove`)
    (`AIBlueprintHelperLibrary.SimpleMoveToActor` (`self.GetController`) (`/Game/Blueprint/FunctionLibrary/FCL_GetCharacter.GetCharacterAs`))
    (else
      (`Controller.StopMovement` (`self.GetController`)))))

(event `self.Sphere.OnComponentBeginOverlap`
  (params (OverlappedComponent :type "PrimitiveComponent Object Reference") (OtherActor :type "Actor Object Reference") (OtherComp :type "PrimitiveComponent Object Reference") (OtherBodyIndex :type Integer) (bFromSweep :type Boolean) (SweepResult :type "HitResult Structure (by ref)"))
  (cast `/Game/Blueprint/ThirdPersonCharacter` OtherActor)
  (`/Game/Blueprint/BP_PlayerController.ChangeLife` (`/Game/Blueprint/FunctionLibrary/FCL_GetController.GetControllerAs`) (`self.dammage`)))

(fn `UserConstructionScript`
  (`parent.UserConstructionScript`))