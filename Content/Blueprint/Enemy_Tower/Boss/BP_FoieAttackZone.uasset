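; BP_FoieAttackZone is a short-lived damage sphere in the Foie boss folder that lowers the player's life.
; With a valid Parent, the sphere follows the parent's AttackZone every tick, damages the first player to begin overlapping, then destroys itself.
; Without a Parent, it damages players already overlapping after a tiny startup delay and expires sooner.
; Damage goes through ChangeLife on the player's controller.
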(event `self.ReceiveBeginPlay`
  (`KismetSystemLibrary.Delay` 0.01)
  (`self.parent`
    (:`then`
      (`self.SetLifeSpan` 0.3))
    (:`else`
      (`self.SetLifeSpan` 0.1)
      (for _array_element (`PrimitiveComponent.GetOverlappingActors` (`self.Sphere`) "/Game/Blueprint/ThirdPersonCharacter.ThirdPersonCharacter_C")
        (cast `/Game/Blueprint/ThirdPersonCharacter` _array_element)
        (`/Game/Blueprint/BP_PlayerController.ChangeLife` (`/Game/Blueprint/FunctionLibrary/FCL_GetController.GetControllerAs`) (* (`self.dammageToPlayer`) -1))))))

(event `self.ReceiveTick`
  (params (DeltaSeconds :type "Float (single-precision)"))
  (bind _parent (`self.parent`)
    (:`then`
      (`SceneComponent.K2_SetWorldTransform` (`self.Sphere`) (`SceneComponent.K2_GetComponentToWorld` (`/Game/Blueprint/Enemy_Tower/Boss/BP_BossFoie.AttackZone` _parent)) false false))
    (:`else`)))

(event `self.Sphere.OnComponentBeginOverlap`
  (params (OverlappedComponent :type "PrimitiveComponent Object Reference") (OtherActor :type "Actor Object Reference") (OtherComp :type "PrimitiveComponent Object Reference") (OtherBodyIndex :type Integer) (bFromSweep :type Boolean) (SweepResult :type "HitResult Structure (by ref)"))
  (`self.parent`
    (:`then`
      (cast `/Game/Blueprint/ThirdPersonCharacter` OtherActor)
      (`/Game/Blueprint/BP_PlayerController.ChangeLife` (`/Game/Blueprint/FunctionLibrary/FCL_GetController.GetControllerAs`) (* (`self.dammageToPlayer`) -1))
      (`self.K2_DestroyActor`))
    (:`else`)))

(fn `UserConstructionScript`)