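; Boss enemy Foie, which chases the player and triggers BP_EndGame actors and a UI system update through AddEffectDead.
; Player overlap with TriggerZone halts movement and picks one of three attacks: single hit, triple hit with forward launches, or dash.
; Attacks spawn timed BP_FoieAttackZone damage actors at the hidden AttackZone.
; While stopped, Tick runs Actions to face the player and drive the dash, using Delays and state flags.
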(event `self.ReceiveBeginPlay`
  (`SceneComponent.SetVisibility` (`self.AttackZone`) false false)
  (set `self.maxLife` 4)
  (`self.ResetStatsEnemy`)
  (set `self.ignorePush` true))

(event `self.ReceiveTick`
  (params (DeltaSeconds :type "Float (single-precision)"))
  (if (`self.canMove`)
    (`AIBlueprintHelperLibrary.SimpleMoveToActor` (`self.GetController`) (`/Game/Blueprint/FunctionLibrary/FCL_GetCharacter.GetCharacterAs`))
    (else
      (`Controller.StopMovement` (`self.GetController`))
      (`self.Actions`))))

(event `self.TriggerZone.OnComponentBeginOverlap`
  (params (OverlappedComponent :type "PrimitiveComponent Object Reference") (OtherActor :type "Actor Object Reference") (OtherComp :type "PrimitiveComponent Object Reference") (OtherBodyIndex :type Integer) (bFromSweep :type Boolean) (SweepResult :type "HitResult Structure (by ref)"))
  (cast `/Game/Blueprint/ThirdPersonCharacter` OtherActor)
  (if (not (`self.inAttack`))
    (set `self.canMove` false)
    (set `self.inAttack` true)
    (`self.SelectRandomAction`)))

(event `SelectRandomAction`
  (set `self.currentAction` (`KismetMathLibrary.RandomInteger` 3))
  (`|ExecutionSequence`
    (:`then_0`
      (if (== (`self.currentAction`) 0)
        (`KismetSystemLibrary.Delay` 0.5)
        (bind _returnvalue (`|SpawnActorFromClass` "/Game/Blueprint/Enemy_Tower/Boss/BP_FoieAttackZone.BP_FoieAttackZone_C" (`SceneComponent.K2_GetComponentToWorld` (`self.AttackZone`)) "Undefined" "OverrideRootScale" null null))
        (set `/Game/Blueprint/Enemy_Tower/Boss/BP_FoieAttackZone.dammageToPlayer` 17 _returnvalue)
        (`KismetSystemLibrary.Delay` 0.2)
        (set `self.canMove` true)
        (set `self.inAttack` false)))
    (:`then_1`
      (if (== (`self.currentAction`) 1)
        (`KismetSystemLibrary.Delay` 1.0)
        (set `self.rotateToPlayerTripleAtk` false)
        (bind _returnvalue_2 (`|SpawnActorFromClass` "/Game/Blueprint/Enemy_Tower/Boss/BP_FoieAttackZone.BP_FoieAttackZone_C" (`SceneComponent.K2_GetComponentToWorld` (`self.AttackZone`)) "Undefined" "OverrideRootScale" null null))
        (set `/Game/Blueprint/Enemy_Tower/Boss/BP_FoieAttackZone.dammageToPlayer` 5 _returnvalue_2)
        (`self.LaunchCharacter` (* (`SceneComponent.GetForwardVector` (`self.CapsuleComponent`)) 1500.0))
        (`KismetSystemLibrary.Delay` 0.5)
        (bind _returnvalue_3 (`|SpawnActorFromClass` "/Game/Blueprint/Enemy_Tower/Boss/BP_FoieAttackZone.BP_FoieAttackZone_C" (`SceneComponent.K2_GetComponentToWorld` (`self.AttackZone`)) "Undefined" "OverrideRootScale" null null))
        (set `/Game/Blueprint/Enemy_Tower/Boss/BP_FoieAttackZone.dammageToPlayer` 5 _returnvalue_3)
        (`self.LaunchCharacter` (* (`SceneComponent.GetForwardVector` (`self.CapsuleComponent`)) 1500.0))
        (`KismetSystemLibrary.Delay` 0.5)
        (bind _returnvalue_4 (`|SpawnActorFromClass` "/Game/Blueprint/Enemy_Tower/Boss/BP_FoieAttackZone.BP_FoieAttackZone_C" (`SceneComponent.K2_GetComponentToWorld` (`self.AttackZone`)) "Undefined" "OverrideRootScale" null null))
        (set `/Game/Blueprint/Enemy_Tower/Boss/BP_FoieAttackZone.dammageToPlayer` 5 _returnvalue_4)
        (`KismetSystemLibrary.Delay` 0.5)
        (set `self.canMove` true)
        (set `self.inAttack` false)))
    (:`then_2`
      (if (== (`self.currentAction`) 2)
        (`KismetSystemLibrary.Delay` 1.0)
        (bind _returnvalue_5 (`|SpawnActorFromClass` "/Game/Blueprint/Enemy_Tower/Boss/BP_FoieAttackZone.BP_FoieAttackZone_C" (`SceneComponent.K2_GetComponentToWorld` (`self.AttackZone`)) "Undefined" "OverrideRootScale" null null))
        (set `/Game/Blueprint/Enemy_Tower/Boss/BP_FoieAttackZone.parent` self _returnvalue_5)
        (set `/Game/Blueprint/Enemy_Tower/Boss/BP_FoieAttackZone.dammageToPlayer` 20 _returnvalue_5)))
    (:`then_3`
      (`self.Actions`))))

(event `Actions`
  (`|ExecutionSequence`
    (:`then_0`
      (if (== (`self.currentAction`) 0)
        (`self.K2_SetActorRotation` (`KismetMathLibrary.FindLookAtRotation` (`self.K2_GetActorLocation`) (`self.K2_GetActorLocation` (`/Game/Blueprint/FunctionLibrary/FCL_GetCharacter.GetCharacterAs`))))
        (`KismetSystemLibrary.Delay` 1.0)))
    (:`then_1`
      (if (== (`self.currentAction`) 1)
        (if (`self.rotateToPlayerTripleAtk`)
          (`self.K2_SetActorRotation` (`KismetMathLibrary.FindLookAtRotation` (`self.K2_GetActorLocation`) (`self.K2_GetActorLocation` (`/Game/Blueprint/FunctionLibrary/FCL_GetCharacter.GetCharacterAs`))))
          (`KismetSystemLibrary.Delay` 1.0))))
    (:`then_2`
      (if (== (`self.currentAction`) 2)
        (if (`self.inDash`)
          (`self.K2_SetActorLocation` (+ (`self.K2_GetActorLocation`) (* (`self.GetActorForwardVector`) 15.0)))
          (`KismetSystemLibrary.Delay` 0.3)
          (set `self.canMove` true)
          (set `self.inAttack` false)
          (set `self.inDash` false)
          (else
            (`self.K2_SetActorRotation` (`KismetMathLibrary.FindLookAtRotation` (`self.K2_GetActorLocation`) (`self.K2_GetActorLocation` (`/Game/Blueprint/FunctionLibrary/FCL_GetCharacter.GetCharacterAs`))))
            (`KismetSystemLibrary.Delay` 1.0)
            (set `self.inDash` true)))))))

(fn `AddEffectDead`
  (bind _outactors (`GameplayStatics.GetAllActorsOfClass` "/Game/Blueprint/MapDetectZone/BP_EndGame.BP_EndGame_C"))
  (for _array_element _outactors
    (`/Game/Blueprint/MapDetectZone/BP_EndGame.EndGame` _array_element)
    (`/Game/Blueprint/WBP_UISystem.setUISystem` (`/Game/Blueprint/BP_PlayerController.uiSystem` (`/Game/Blueprint/FunctionLibrary/FCL_GetController.GetControllerAs`)) (`self.dammageToSystem`))))

(fn `UserConstructionScript`
  (`parent.UserConstructionScript`))