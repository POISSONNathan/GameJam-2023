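; Bomb enemy that chases the player and explodes shortly after the player enters its trigger zone.
; While CanMove is set, Tick moves it toward the character until an overlap with ThirdPersonCharacter sets Explode.
; It then swells its mesh every tick during a short Delay, spawns BP_EnemyBombZone and an explosion effect, and destroys itself.
; BeginPlay hides the Sphere, sets MaxLife and resets enemy stats.
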(event `self.ReceiveBeginPlay`
  (`SceneComponent.SetVisibility` (`self.Sphere`) false false)
  (set `self.maxLife` 3)
  (`self.ResetStatsEnemy`))

(event `self.ReceiveTick`
  (params (DeltaSeconds :type "Float (single-precision)"))
  (bind _mesh (`self.Mesh`))
  (if (`self.canMove`)
    (if (`self.explode`)
      (`SceneComponent.SetWorldScale3D` _mesh (+ (`SceneComponent.K2_GetComponentScale` _mesh) (0.005 0.005 0.005)))
      (`KismetSystemLibrary.Delay` 1.0)
      (`|SpawnActorFromClass` "/Game/Blueprint/Enemy_Tower/EnemyBomb/BP_EnemyBombZone.BP_EnemyBombZone_C" (`SceneComponent.K2_GetComponentToWorld` (`self.Sphere`)) "Undefined" "OverrideRootScale" null null)
      (`GameplayStatics.SpawnEmitterAtLocation` "/Game/StarterContent/Particles/P_Explosion.P_Explosion" (`self.K2_GetActorLocation`))
      (`self.K2_DestroyActor`)
      (else
        (`AIBlueprintHelperLibrary.SimpleMoveToActor` (`self.GetController`) (`/Game/Blueprint/FunctionLibrary/FCL_GetCharacter.GetCharacterAs`))))))

(event `self.TriggerZone.OnComponentBeginOverlap`
  (params (OverlappedComponent :type "PrimitiveComponent Object Reference") (OtherActor :type "Actor Object Reference") (OtherComp :type "PrimitiveComponent Object Reference") (OtherBodyIndex :type Integer) (bFromSweep :type Boolean) (SweepResult :type "HitResult Structure (by ref)"))
  (cast `/Game/Blueprint/ThirdPersonCharacter` OtherActor)
  (set `self.explode` true))

(fn `UserConstructionScript`
  (`parent.UserConstructionScript`))