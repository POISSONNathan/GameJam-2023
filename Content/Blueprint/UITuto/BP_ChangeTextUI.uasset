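; BP_ChangeTextUI is a trigger volume that changes the tutorial text on screen when the player walks into it.
; A Box overlap by ThirdPersonCharacter pushes the actor's CurrentText to the controller's UiSystem through SetTextTuto.
; The actor then destroys itself, first waiting and clearing the text when LastMessage is set.
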(event `self.Box.OnComponentBeginOverlap`
  (params (OverlappedComponent :type "PrimitiveComponent Object Reference") (OtherActor :type "Actor Object Reference") (OtherComp :type "PrimitiveComponent Object Reference") (OtherBodyIndex :type Integer) (bFromSweep :type Boolean) (SweepResult :type "HitResult Structure (by ref)"))
  (cast `/Game/Blueprint/ThirdPersonCharacter` OtherActor)
  (`/Game/Blueprint/WBP_UISystem.setTextTuto` (`/Game/Blueprint/BP_PlayerController.uiSystem` (`/Game/Blueprint/FunctionLibrary/FCL_GetController.GetControllerAs`)) (`self.currentText`))
  (if (`self.lastMessage`)
    (`KismetSystemLibrary.Delay` 5.0)
    (`/Game/Blueprint/WBP_UISystem.setTextTuto` (`/Game/Blueprint/BP_PlayerController.uiSystem` (`/Game/Blueprint/FunctionLibrary/FCL_GetController.GetControllerAs`)) "")
    (`self.K2_DestroyActor`)
    (else
      (`self.K2_DestroyActor`))))

(fn `UserConstructionScript`)