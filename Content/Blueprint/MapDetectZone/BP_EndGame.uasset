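; BP_EndGame is an end-of-game camera actor that takes over the player's view and clears the level of enemies.
; EndGame blends the view to this actor, disables character input, then destroys every BP_Enemy.
; The Delay after each destroy sits inside the loop, so it does not stagger the removals.
; Tick plays a world camera shake at its camera's location every frame, independent of EndGame.
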(event `EndGame`
  (`PlayerController.SetViewTargetWithBlend` (`/Game/Blueprint/FunctionLibrary/FCL_GetController.GetControllerAs`) self 1.0 "VTBlend_Linear" 0.0 false)
  (`self.DisableInput` (`/Game/Blueprint/FunctionLibrary/FCL_GetCharacter.GetCharacterAs`) null)
  (bind _outactors (`GameplayStatics.GetAllActorsOfClass` "/Game/Blueprint/Enemy_Tower/BP_Enemy.BP_Enemy_C"))
  (for _array_element _outactors
    (`self.K2_DestroyActor` _array_element)
    (`KismetSystemLibrary.Delay` 1.0)))

(event `self.ReceiveTick`
  (params (DeltaSeconds :type "Float (single-precision)"))
  (`GameplayStatics.PlayWorldCameraShake` "/Game/Blueprint/MapDetectZone/CS_ShakeCam.CS_ShakeCam_C" (`SceneComponent.K2_GetComponentLocation` (`self.Camera`)) 500.0))

(fn `UserConstructionScript`)