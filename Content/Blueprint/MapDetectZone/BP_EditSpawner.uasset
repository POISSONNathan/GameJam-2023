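; BP_EditSpawner is a map trigger box that switches enemy spawning on or off when the ThirdPersonCharacter enters it.
; On overlap it copies Activate to the controller's EnemyCanSpawn, resets the enemy count and calls SpawnEnemy.
; An activating trigger then destroys itself.
; A deactivating one clears all BP_Enemy actors and, if SpawnBoss is set, spawns BP_BossFoie, passes it LocationSpawnerTP and self-destructs.
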(event `self.Box.OnComponentBeginOverlap`
  (params (OverlappedComponent :type "PrimitiveComponent Object Reference") (OtherActor :type "Actor Object Reference") (OtherComp :type "PrimitiveComponent Object Reference") (OtherBodyIndex :type Integer) (bFromSweep :type Boolean) (SweepResult :type "HitResult Structure (by ref)"))
  (bind _asbp_player_controller (`/Game/Blueprint/FunctionLibrary/FCL_GetController.GetControllerAs`))
  (cast `/Game/Blueprint/ThirdPersonCharacter` OtherActor)
  (bind _output_get (set `/Game/Blueprint/BP_PlayerController.enemyCanSpawn` (`self.activate`) _asbp_player_controller))
  (set `/Game/Blueprint/BP_PlayerController.numberEnemyOnMap` 0 _asbp_player_controller)
  (`/Game/Blueprint/BP_PlayerController.SpawnEnemy` _asbp_player_controller)
  (set `/Game/Blueprint/BP_PlayerController.canSpawn` true _asbp_player_controller)
  (if _output_get
    (`self.K2_DestroyActor`)
    (else
      (bind _outactors (`GameplayStatics.GetAllActorsOfClass` "/Game/Blueprint/Enemy_Tower/BP_Enemy.BP_Enemy_C"))
      (for _array_element _outactors
        (`self.K2_DestroyActor` _array_element))
      (if (`self.spawnBoss`)
        (bind _returnvalue (`AIBlueprintHelperLibrary.SpawnAIFromClass` "/Game/Blueprint/Enemy_Tower/Boss/BP_BossFoie.BP_BossFoie_C" null (`self.K2_GetActorLocation` (`self.location`)) (struct) false null))
        (bind _asbp_boss_foie (cast `/Game/Blueprint/Enemy_Tower/Boss/BP_BossFoie` _returnvalue))
        (set `/Game/Blueprint/Enemy_Tower/Boss/BP_BossFoie.locationSpawnerTP` (`self.locationSpawnerTP`) _asbp_boss_foie)
        (`self.K2_DestroyActor`)))))

(fn `UserConstructionScript`)