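; BP_PushZone is an actor that pushes nearby enemies away when it spawns.
; After a very short delay on BeginPlay, it gets the BP_Enemy actors overlapping its Sphere and calls GetPushed on each, as a one-time check.
; Every Tick it snaps the Sphere to the world transform of the character's PushZone component, without sweep or teleport.
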(event `self.ReceiveTick`
  (params (DeltaSeconds :type "Float (single-precision)"))
  (`SceneComponent.K2_SetWorldTransform` (`self.Sphere`) (`SceneComponent.K2_GetComponentToWorld` (`/Game/Blueprint/ThirdPersonCharacter.PushZone` (`/Game/Blueprint/FunctionLibrary/FCL_GetCharacter.GetCharacterAs`))) false false))

(event `self.ReceiveBeginPlay`
  (`KismetSystemLibrary.Delay` 0.01)
  (for _array_element (`PrimitiveComponent.GetOverlappingActors` (`self.Sphere`) "/Game/Blueprint/Enemy_Tower/BP_Enemy.BP_Enemy_C")
    (bind _asbp_enemy (cast `/Game/Blueprint/Enemy_Tower/BP_Enemy` _array_element))
    (`/Game/Blueprint/Enemy_Tower/BP_Enemy.GetPushed` _asbp_enemy)))

(fn `UserConstructionScript`)