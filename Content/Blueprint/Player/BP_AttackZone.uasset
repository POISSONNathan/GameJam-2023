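; BP_AttackZone is an attack hit area that damages enemies and towers inside its sphere.
; Shortly after BeginPlay, it makes a single overlap query per target type and calls TakeDammage with a fixed amount on each BP_Enemy and BP_Tower found.
; Each Tick snaps the sphere to the character's AttackZone transform without sweeping.
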(event `self.ReceiveTick`
  (params (DeltaSeconds :type "Float (single-precision)"))
  (`SceneComponent.K2_SetWorldTransform` (`self.Sphere`) (`SceneComponent.K2_GetComponentToWorld` (`/Game/Blueprint/ThirdPersonCharacter.AttackZone` (`/Game/Blueprint/FunctionLibrary/FCL_GetCharacter.GetCharacterAs`))) false false))

(event `self.ReceiveBeginPlay`
  (`KismetSystemLibrary.Delay` 0.01)
  (for _array_element (`PrimitiveComponent.GetOverlappingActors` (`self.Sphere`) "/Game/Blueprint/Enemy_Tower/BP_Enemy.BP_Enemy_C")
    (bind _asbp_enemy (cast `/Game/Blueprint/Enemy_Tower/BP_Enemy` _array_element))
    (`/Game/Blueprint/Enemy_Tower/BP_Enemy.TakeDammage` _asbp_enemy 2))
  (for _array_element_2 (`PrimitiveComponent.GetOverlappingActors` (`self.Sphere`) "/Game/Blueprint/Enemy_Tower/Tower/BP_Tower.BP_Tower_C")
    (bind _asbp_tower (cast `/Game/Blueprint/Enemy_Tower/Tower/BP_Tower` _array_element_2))
    (`/Game/Blueprint/Enemy_Tower/Tower/BP_Tower.TakeDammage` _asbp_tower 2)))

(fn `UserConstructionScript`)